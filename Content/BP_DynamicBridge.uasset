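; Dynamic-mesh bridge actor that procedurally builds a wavy span and animates it extending and retracting over time.
; GenerateBridge appends a box subdivided along Y by Resolution, then applies horizontal and vertical sine-wave deformations.
; The construction script builds it at full Length, while Tick rebuilds it every frame with a cosine-driven length between zero and Length.
; Each rebuild uses temporary compute meshes, copied into the actor and then released.
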(event `self.ReceiveTick`
  (params (DeltaSeconds :type "Float (single-precision)"))
  (bind _returnvalue (`self.AllocateComputeMesh`))
  (bind _updatedinputmesh (`self.GenerateBridge` _returnvalue (* (/ (+ (`KismetMathLibrary.Cos` (* (`self.GetGameTimeSinceCreation`) 0.5)) 1.0) 2.0) (`self.Length`))))
  (`self.CopyFromMesh` _updatedinputmesh)
  (`self.ReleaseAllComputeMeshes`))

(event `self.ReceiveBeginPlay`
  (`self.SetActorTickInterval` 0.0))

(fn `GenerateBridge`
  (params (InputMesh :type "GeneratedMesh Object Reference") (UseLength :type "Float (double-precision)"))
  (returns (UpdatedInputMesh :type "GeneratedMesh Object Reference"))
  (bind _returnvalue (`GeneratedMesh.AppendAxisBox` InputMesh (-50.0 -50.0 -50.0) (`KismetMathLibrary.MakeVector` (`self.Width`) UseLength (`self.Height`)) 0 (`KismetMathLibrary.FCeil` (/ UseLength (`self.Resolution`))) 0))
  (bind _returnvalue_2 (`GeneratedMeshDeformersLibrary.DeformMeshAxisSinWave1D` _returnvalue (`self.MagnitudeHorz`) (/ 1.0 (`self.FrequencyHorz`)) 0.0 (0.0 1.0 0.0) (1.0 0.0 0.0)))
  (bind _returnvalue_3 (`GeneratedMeshDeformersLibrary.DeformMeshAxisSinWave1D` _returnvalue_2 (`self.MagnitudeVert`) (/ 1.0 (`self.FrequencyVert`)) 0.0 (0.0 1.0 0.0)))
  (return _returnvalue_3))

(fn `UserConstructionScript`
  (bind _returnvalue (`self.AllocateComputeMesh`))
  (bind _updatedinputmesh (`self.GenerateBridge` _returnvalue (`self.Length`)))
  (`self.CopyFromMesh` self _updatedinputmesh false false)
  (`self.ReleaseAllComputeMeshes`))